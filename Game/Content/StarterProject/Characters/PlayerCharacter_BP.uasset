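; Player character Blueprint that gives each character one of three rigged human skeletal meshes.
; BeginPlay applies the mesh for the current ModelIndex, then picks a random index only when running on a dedicated server.
; ModelIndex uses a RepNotify that calls UpdateMesh, which selects the mesh by index and sets it with a pose reinit.
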(event `self.ReceiveBeginPlay`
  (`self.UpdateMesh`)
  (if (`KismetSystemLibrary.IsDedicatedServer`)
    (set `self.ModelIndex` (`KismetMathLibrary.RandomIntegerInRange` 0 2))))

(fn `OnRep_ModelIndex`
  (`self.UpdateMesh`))

(fn `UpdateMesh`
  (`SkinnedMeshComponent.SetSkinnedAssetAndUpdate` (`self.Mesh`) (select `int` (`self.ModelIndex`) :`0` "/Game/Scanned3DPeoplePack/RP_Character/rp_carla_rigged_001_Mobile_ue4/rp_carla_rigged_001_Mobile_ue4.rp_carla_rigged_001_Mobile_ue4" :`1` "/Game/Scanned3DPeoplePack/RP_Character/rp_claudia_rigged_002_Mobile_ue4/rp_claudia_rigged_002_Mobile_ue4.rp_claudia_rigged_002_Mobile_ue4" :`2` "/Game/Scanned3DPeoplePack/RP_Character/rp_eric_rigged_001_Mobile_ue4/rp_eric_rigged_001_Mobile_ue4.rp_eric_rigged_001_Mobile_ue4" :!type "SkeletalMesh Object Reference") true))

(fn `UserConstructionScript`)