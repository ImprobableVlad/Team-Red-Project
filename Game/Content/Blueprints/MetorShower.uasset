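; MetorShower is a meteor shower Blueprint that repeatedly spawns Meteor actors high above random players, only on a dedicated server.
; From BeginPlay, a delay via the DelayTime helper precedes a random player pick and a loop spawning meteors at random horizontal offsets scaled by Radius.
; The loop body wires back into the delay to keep the shower going.
; The cycle ends if no players are found.
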(event `self.ReceiveBeginPlay`
  (if (`KismetSystemLibrary.IsDedicatedServer`)
    (bind _delay (`self.DelayTime` 1 1 :!label _label))
    (`KismetSystemLibrary.Delay` (`KismetMathLibrary.Conv_IntToDouble` _delay))
    (bind (_are_players _random_player) (`/Game/PlayerFunctions.Get Random Player` self))
    (if _are_players
      (for _ (range 3)
        (`|SpawnActorFromClass` "/Game/Blueprints/Meteor.Meteor_C" (`KismetMathLibrary.Conv_VectorToTransform` (+ (+ (`self.K2_GetActorLocation` _random_player) (0.0 0.0 1000.0)) (`KismetMathLibrary.MakeVector` (.x (* (`KismetMathLibrary.RandomUnitVector`) (`self.Radius`))) (.y (* (`KismetMathLibrary.RandomUnitVector`) (`self.Radius`))) 6000.0))) "Undefined" "OverrideRootScale" null null)
        (`KismetSystemLibrary.PrintString` "spawn meteors" true true (struct :`R` 1.0 :`G` 0.395744 :`B` 0.75711 :`A` 1.0))
        (goto _label)))))

(fn `DelayTime`
  (params (Min :type Integer) (Max :type Integer))
  (returns (Delay :type Integer))
  (return (`KismetMathLibrary.RandomIntegerInRange` Min Max)))

(fn `UserConstructionScript`)