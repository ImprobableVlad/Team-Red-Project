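; BP_MountainActor is a mountain actor that, on a dedicated server, picks a random seed at BeginPlay, then calls UpdateMountain and SpawnPalms.
; SpawnPalms is an unfinished stub that loops over PalmAmount without spawning anything.
; RandomMountainRaycast traces from high altitude to zero height at random XY against world objects and stores the hit location.
; Nothing here calls that raycast, and its retry loop and return are unconnected.
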(event `self.ReceiveBeginPlay`
  (if (`KismetSystemLibrary.IsDedicatedServer`)
    (set `self.Seed` (`KismetMathLibrary.RandomInteger` 2000000000))
    (`self.UpdateMountain`)
    (`self.SpawnPalms`)))

(event `self.ReceiveTick`
  (params (DeltaSeconds :type "Float (single-precision)")))

(fn `RandomMountainRaycast`
  (returns (NewParam :type "Vector Structure"))
  (locals (Hit :type "Vector Structure"))
  (bind _returnvalue (`KismetMathLibrary.RandomFloatInRange` -15000.0 15000.0))
  (bind _returnvalue_2 (`KismetMathLibrary.RandomFloatInRange` -15000.0 15000.0))
  (bind (_outhit _returnvalue_3) (`KismetSystemLibrary.LineTraceSingleForObjects` (`KismetMathLibrary.MakeVector` _returnvalue_2 _returnvalue 150000.0) (`KismetMathLibrary.MakeVector` _returnvalue_2 _returnvalue) (`|MakeArray` "ObjectTypeQuery1" "ObjectTypeQuery2" :!type "EObjectTypeQuery Enum")))
  (set `local.Hit` (`.Location` (`GameplayStatics.BreakHitResult` _outhit))))

(fn `SpawnPalms`
  (for _ (range (+ (`self.PalmAmount`) 1))
    (while false
      _)))

(fn `UserConstructionScript`)