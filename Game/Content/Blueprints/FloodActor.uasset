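; Flood actor that gradually raises the level's water, represented by an actor tagged "water".
; On BeginPlay it finds the first tagged actor and records its starting Z.
; Each Tick lifts it at a constant rate derived from the height difference over FloodInterval, scaled by delta time and capped at EndHeight.
; EndPlay moves the water actor to the world origin rather than back to its starting height.
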(event `self.ReceiveBeginPlay`
  (bind _outactors (`GameplayStatics.GetAllActorsWithTag` "water"))
  (bind _output (`|GetArrayItem` _outactors))
  (bind _output_get (set `self.WaterActor` _output))
  (if (not (`KismetSystemLibrary.IsValid` _output_get))
    (`KismetSystemLibrary.PrintString` "No actor with tag \"water\" found!"))
  (set `self.StartHeight` (.z (`self.K2_GetActorLocation` _output))))

(event `self.ReceiveTick`
  (params (DeltaSeconds :type "Float (single-precision)"))
  (bind _wateractor (`self.WaterActor`))
  (if (`KismetSystemLibrary.IsValid` _wateractor)
    (`self.K2_SetActorLocation` (`self.WaterActor`) (`KismetMathLibrary.MakeVector` (.x (`self.K2_GetActorLocation` _wateractor)) (.y (`self.K2_GetActorLocation` _wateractor)) (`KismetMathLibrary.FMin` (+ (* DeltaSeconds (/ (- (`self.EndHeight`) (`self.StartHeight`)) (`self.FloodInterval`))) (.z (`self.K2_GetActorLocation` _wateractor))) (`self.EndHeight`))) false false)
    (else
      (`KismetSystemLibrary.PrintString` "No valid water actor"))))

(event `self.ReceiveEndPlay`
  (params (EndPlayReason :type "EEndPlayReason Enum" :default "Destroyed"))
  (`self.K2_SetActorLocation` (`self.WaterActor`) (0.0 0.0 0.0) false false))

(fn `UserConstructionScript`)