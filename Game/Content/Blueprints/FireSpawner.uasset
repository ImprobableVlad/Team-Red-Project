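; FireSpawner is an actor that keeps spawning Brazier actors around the players for as long as it runs.
; From BeginPlay it loops forever, waiting a random whole number of seconds between Min and Max via the DelayTime function.
; After each wait it averages the locations of all PlayerController actors and spawns a Brazier at a random navigable point within a fixed radius of that average.
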(event `self.ReceiveBeginPlay`
  (bind _delay (`self.DelayTime` (`self.Min`) (`self.Max`) :!label _label))
  (`KismetSystemLibrary.Delay` (`KismetMathLibrary.Conv_IntToDouble` _delay))
  (bind _outactors (`GameplayStatics.GetAllActorsOfClass` "/Script/Engine.PlayerController"))
  (bind _returnvalue (`GameplayStatics.GetActorArrayAverageLocation` _outactors))
  (`|SpawnActorFromClass` "/Game/Blueprints/Brazier.Brazier_C" (`KismetMathLibrary.Conv_VectorToTransform` (`NavigationSystemV1.K2_GetRandomLocationInNavigableRadius` _returnvalue 1000.0 null null)) "Undefined" "OverrideRootScale" null null)
  (goto _label))

(fn `DelayTime`
  (params (Min :type Integer) (Max :type Integer))
  (returns (Delay :type Integer))
  (return (`KismetMathLibrary.RandomIntegerInRange` Min Max)))

(fn `UserConstructionScript`)