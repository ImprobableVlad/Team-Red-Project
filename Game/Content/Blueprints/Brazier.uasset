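; Brazier is a fire hazard that damages an overlapping player, applying the damage to the player's controller, and spreads across nearby cubes.
; On dedicated servers, a delayed BeginPlay sphere search finds unlit Cube_BP actors, marks them on fire and spawns another Brazier at each, chaining the spread.
; A second Delay inside the loop precedes enabling cube physics, so that latent step does not run separately per cube.
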(event `self.ReceiveActorBeginOverlap`
  (params (OtherActor :type "Actor Object Reference"))
  (bind _asplayer_character_bp (cast `/Game/StarterProject/Characters/PlayerCharacter_BP` OtherActor))
  (`GameplayStatics.ApplyDamage` (`Pawn.GetController` _asplayer_character_bp) 20.0))

(event `self.ReceiveBeginPlay`
  (if (`KismetSystemLibrary.IsDedicatedServer`)
    (`KismetSystemLibrary.Delay` 2.0)
    (bind _outactors (`KismetSystemLibrary.SphereOverlapActors` (`self.K2_GetActorLocation`) 500.0 (`|MakeArray` "ObjectTypeQuery7" :!type "EObjectTypeQuery Enum") "/Game/Cube_BP.Cube_BP_C"))
    (for _array_element _outactors
      (bind _ascube_bp (cast `/Game/Cube_BP` _array_element))
      (if (not (`/Game/Cube_BP.IsOnFire` _ascube_bp))
        (`KismetSystemLibrary.PrintString` "FOUND CUBE" true true (struct :`R` 0.220451 :`G` 0.092793 :`B` 1.0 :`A` 1.0))
        (`|SpawnActorFromClass` "Brazier_C" (`KismetMathLibrary.Conv_VectorToTransform` (`self.K2_GetActorLocation` _array_element)) "AlwaysSpawn" "OverrideRootScale" null null)
        (bind _ascube_bp_2 (cast `/Game/Cube_BP` _array_element))
        (set `/Game/Cube_BP.IsOnFire` true _ascube_bp_2)
        (`KismetSystemLibrary.Delay` 1.0)
        (`PrimitiveComponent.SetSimulatePhysics` (`/Game/Cube_BP.Cube` _ascube_bp_2) true)))))

(event `self.ReceiveTick`
  (params (DeltaSeconds :type "Float (single-precision)")))

(fn `UserConstructionScript`)