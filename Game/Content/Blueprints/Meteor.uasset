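; Meteor actor that explodes when its Sphere component hits something.
; Every hit attaches an explosion particle to the sphere, while a HasExploded flag limits the ExplodeWolfExplosion actor spawn at the meteor's location to the first hit.
; Impact does not destroy the meteor; a counter incremented on Tick destroys it after a fixed number of frames, so its lifetime depends on frame rate.
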(event `self.ReceiveBeginPlay`
  (set `self.TimeAlive` 0))

(event `self.ReceiveTick`
  (params (DeltaSeconds :type "Float (single-precision)"))
  (bind _result (`/Engine/EditorBlueprintResources/StandardMacros.IncrementInt` (`self.TimeAlive`))
    (:`  `
      (bind _output_get (set `self.TimeAlive` _result))
      (`/Engine/EditorBlueprintResources/StandardMacros.CompareInt` _output_get 1000
        (:`>`
          (if true
            (`self.K2_DestroyActor`)))))))

(event `self.Sphere.OnComponentHit`
  (params (HitComponent :type "PrimitiveComponent Object Reference") (OtherActor :type "Actor Object Reference") (OtherComp :type "PrimitiveComponent Object Reference") (NormalImpulse :type "Vector Structure") (Hit :type "HitResult Structure (by ref)"))
  (`GameplayStatics.SpawnEmitterAttached` "/Game/StarterContent/Particles/P_Explosion.P_Explosion" HitComponent)
  (if (not (`self.HasExploded`))
    (`|SpawnActorFromClass` "/Game/ExplodeWolfExplosion.ExplodeWolfExplosion_C" (`KismetMathLibrary.Conv_VectorToTransform` (`self.K2_GetActorLocation`)) "Undefined" "OverrideRootScale" null null)
    (set `self.HasExploded` true)))

(fn `UserConstructionScript`)