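; Player controller for a round-based game of block building and surviving disasters, handling build mode, health and death.
; Key 1 toggles build mode, which frees the cursor and locks the camera; clicks spawn grid-snapped Cube_BP blocks or delete those the player's pawn instigated.
; Damage reaching zero health ragdolls the character, and a dedicated server notifies GameManager after a delay.
; Remote instances create the GameInterface widget and forward round and disaster events to it.
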(event `DeleteBlock`
  (params (Object :type "Actor Object Reference"))
  (`self.K2_DestroyActor` Object))

(event `SpawnBlock`
  (params (SpawnTransform :type "Transform Structure") (Instigator :type "Pawn Object Reference"))
  (bind _returnvalue (`|SpawnActorFromClass` "/Game/Cube_BP.Cube_BP_C" SpawnTransform "AlwaysSpawn" "OverrideRootScale" null Instigator))
  (`KismetSystemLibrary.PrintString` (`KismetStringLibrary.Conv_VectorToString` (`self.K2_GetActorLocation` _returnvalue))))

(event `Key|RightMouseButton`
  (params (Key :type "Key Structure"))
  (bind (_hitresult _returnvalue) (`self.GetHitResultUnderCursorForObjects` (`|MakeArray` "ObjectTypeQuery7" :!type "EObjectTypeQuery Enum")))
  (:`Pressed`
    (if (`self.IsPlacing`)
      (if _returnvalue
        (bind _ascube_bp (cast `/Game/Cube_BP` (`.HitActor` (`GameplayStatics.BreakHitResult` _hitresult))))
        (if (== (`self.GetInstigator` _ascube_bp) (`self.K2_GetPawn`))
          (`self.DeleteBlock` _ascube_bp))))))

(event `self.ReceiveBeginPlay`
  (`/Engine/EditorBlueprintResources/ActorMacros.Switch Has Authority`
    (:`Remote`
      (bind _returnvalue (`|CreateWidget` "/Game/GameInterface.GameInterface_C" self))
      (`UserWidget.AddToViewport` _returnvalue 0)
      (set `self.IsPlacing` false))))

(event `Key|LeftMouseButton`
  (params (Key :type "Key Structure"))
  (bind (_bblockinghit _binitialoverlap _time _distance _location _impactpoint _normal) (`GameplayStatics.BreakHitResult` (`self.GetHitResultUnderCursorForObjects` (`|MakeArray` "ObjectTypeQuery1" "ObjectTypeQuery2" "ObjectTypeQuery4" "ObjectTypeQuery6" "ObjectTypeQuery7" :!type "EObjectTypeQuery Enum"))))
  (:`Pressed`
    (if (`self.IsPlacing`)
      (`self.SpawnBlock` (`KismetMathLibrary.Conv_VectorToTransform` (- (* (`KismetMathLibrary.MakeVector` (`KismetMathLibrary.Conv_IntToDouble` (`KismetMathLibrary.Round` (.x (/ (- (+ _location (* _normal 50.0)) (-50.0 -50.0 -50.0)) 100)))) (`KismetMathLibrary.Conv_IntToDouble` (`KismetMathLibrary.Round` (.y (/ (- (+ _location (* _normal 50.0)) (-50.0 -50.0 -50.0)) 100)))) (`KismetMathLibrary.Conv_IntToDouble` (`KismetMathLibrary.Round` (.z (/ (- (+ _location (* _normal 50.0)) (-50.0 -50.0 -50.0)) 100))))) 100) (50.0 50.0 50.0))) (`self.K2_GetPawn`)))))

(event `self.ReceiveAnyDamage`
  (params (Damage :type "Float (single-precision)") (DamageType :type "DamageType Object Reference") (InstigatedBy :type "Controller Object Reference") (DamageCauser :type "Actor Object Reference"))
  (if (not (`self.IsDead`))
    (bind _output_get (set `self.Health` (- (`self.Health`) Damage)))
    (if (<= _output_get 0.0)
      (`self.Die`))))

(event `Key|One`
  (params (Key :type "Key Structure"))
  (:`Pressed`
    (if (`self.IsPlacing`)
      (set `self.IsPlacing` false)
      (`self.ResetCamera`)
      (else
        (set `self.IsPlacing` true)
        (`self.FixCamera`)))))

(event `Die`
  (set `self.IsDead` true)
  (bind _asplayer_character_bp (cast `/Game/StarterProject/Characters/PlayerCharacter_BP` (`self.K2_GetPawn`)))
  (`PrimitiveComponent.SetSimulatePhysics` (`Character.CapsuleComponent` _asplayer_character_bp) true)
  (`SkeletalMeshComponent.SetAllBodiesSimulatePhysics` (`Character.Mesh` _asplayer_character_bp) true)
  (if (`KismetSystemLibrary.IsDedicatedServer`)
    (`KismetSystemLibrary.Delay` 3.0)
    (`/Game/GameManager.PlayerDied` (`self.GameManager`) self)))

(event `FixCamera`
  (set `self.bShowMouseCursor` true)
  (bind _asplayer_character_bp (cast `/Game/StarterProject/Characters/PlayerCharacter_BP` (`self.K2_GetPawn`)))
  (bind _cameraboom (`TeamRedProjectCharacter.CameraBoom` _asplayer_character_bp))
  (set `SpringArmComponent.bUsePawnControlRotation` false _cameraboom)
  (set `SpringArmComponent.bInheritYaw` false _cameraboom)
  (set `SpringArmComponent.bInheritPitch` false _cameraboom)
  (set `SpringArmComponent.bInheritRoll` false _cameraboom)
  (set `TeamRedProjectCharacter.ControllerInputEnabled` false _asplayer_character_bp)
  (`SceneComponent.K2_SetRelativeRotation` _cameraboom (`Pawn.GetControlRotation` _asplayer_character_bp) false false))

(event `ResetCamera`
  (set `self.bShowMouseCursor` false)
  (bind _asplayer_character_bp (cast `/Game/StarterProject/Characters/PlayerCharacter_BP` (`self.K2_GetPawn`)))
  (bind _cameraboom (`TeamRedProjectCharacter.CameraBoom` _asplayer_character_bp))
  (set `SpringArmComponent.bUsePawnControlRotation` true _cameraboom)
  (set `SpringArmComponent.bInheritYaw` true _cameraboom)
  (set `SpringArmComponent.bInheritPitch` true _cameraboom)
  (set `SpringArmComponent.bInheritRoll` true _cameraboom)
  (set `TeamRedProjectCharacter.ControllerInputEnabled` true _asplayer_character_bp))

(event `RoundStarted`
  (params (BuildLength :type "Float (double-precision)") (`Disaster Type` :type String))
  (set `self.Health` 100.0)
  (set `self.IsDead` false)
  (`/Engine/EditorBlueprintResources/ActorMacros.Switch Has Authority`
    (:`Remote`
      (bind _foundwidgets (`WidgetBlueprintLibrary.GetAllWidgetsOfClass` "/Game/GameInterface.GameInterface_C"))
      (for _array_element _foundwidgets
        (`/Game/GameInterface.RoundBeginEvent` _array_element BuildLength `Disaster Type`)))))

(event `BuildingEnded`
  (params (TimeLeft :type "Float (double-precision)"))
  (`/Engine/EditorBlueprintResources/ActorMacros.Switch Has Authority`
    (:`Remote`
      (bind _foundwidgets (`WidgetBlueprintLibrary.GetAllWidgetsOfClass` "/Game/GameInterface.GameInterface_C"))
      (for _array_element _foundwidgets
        (`/Game/GameInterface.DisasterBeginEvent` _array_element TimeLeft)))))

(fn `UserConstructionScript`)